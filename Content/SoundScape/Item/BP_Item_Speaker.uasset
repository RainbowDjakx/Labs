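; BP_Item_Speaker is an interactable speaker item in the SoundScape radio system.
; On BeginPlay it passes its hitbox and MetaSound radio source to its BPCRadio component.
; Interacting signals a speaker hover to the BPCRadioControler component on the player reference.
; The construction script scales the hitbox from a size variable.
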(event EventBeginPlay
  (Default|EventSetHitbox (Variables|Default|GetBPC_Radio) (Variables|Default|GetHitbox))
  (Default|EventSetMetaSound (Variables|Default|GetBPC_Radio) (Variables|Default|GetMS_Radio)))

(event EventFunctionInteract
  (params (Ref_Player :type Bp%20Player%20Object%20Reference) (Over/Select :type Boolean))
  (Variables|Default|SetRef%20Player 0)
  (Default|EventSpeakerHover (Variables|/Game/SoundScape/Player/Bp_Player.Bp_Player_C|GetBPC_RadioControler (Variables|Default|GetRef%20Player)) true))

(fn ConstructionScript
  ;[1 0.9365 0.2371] HitBox Setup
  (Transformation|SetRelativeScale3D (Variables|Default|GetHitbox) (Variables|Default|GetHitBox_Size)))