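; Player Blueprint that switches between a normal camera and a scope camera, showing a frequency display while scoped.
; BeginPlay creates the WB_FrequenceDisplay widget and stores it as the HUD.
; Event_ChangeCamera takes an IsScope flag, toggles which camera is active, adds or removes that HUD from the viewport, and prints the scope state.
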(event Custom|Event_ChangeCamera
  (params (Is_Scope :type Boolean))
  (bind _hud (Variables|Default|GetHUD))
  (if Is_Scope
    (Components|Activation|SetActive (Variables|Default|GetCamera_Scop) true false)
    (Components|Activation|SetActive (Variables|Default|GetCamera) false false)
    (Development|PrintString "Scope Activate")
    (UserInterface|Viewport|AddtoViewport _hud 0)
    (else
      (Components|Activation|SetActive (Variables|Default|GetCamera) true false)
      (Components|Activation|SetActive (Variables|Default|GetCamera_Scop) false false)
      (Development|PrintString "Scope Desactivate")
      (Widget|RemovefromParent _hud))))

(event EventBeginPlay
  (bind _returnvalue (UserInterface|CreateWidget "/Game/SoundScape/Interface/WB_FrequenceDisplay.WB_FrequenceDisplay_C"))
  (Variables|Default|SetHUD _returnvalue))

(fn ConstructionScript)