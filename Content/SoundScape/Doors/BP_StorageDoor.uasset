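; Storage door actor that slides vertically when its open and close events are called.
; A timeline drives the door's relative Z between DoorOpen and DoorClose, playing from the start to open and reversing from the end to close.
; The construction script sets DoorClose from the door's Z, then overwrites it with an offset from the OpenPositioon component; DoorOpen is not assigned in these graphs.
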(event Custom|Event_OpenDoor
  (bind _mouvementvalue (Timeline|Timeline PlayFromStart)
    (:Update
      (Transformation|SetRelativeLocation (Variables|Default|GetDoor) (Math|Vector|MakeVector 0.0 0.0 (Math|Float|Lerp (Variables|Default|GetDoor_Open) (Variables|Default|GetDoor_Close) _mouvementvalue)) false false))))

(event Custom|Event_CloseDoor
  (bind _mouvementvalue (Timeline|Timeline ReverseFromEnd)
    (:Update
      (Transformation|SetRelativeLocation (Variables|Default|GetDoor) (Math|Vector|MakeVector 0.0 0.0 (Math|Float|Lerp (Variables|Default|GetDoor_Open) (Variables|Default|GetDoor_Close) _mouvementvalue)) false false))))

(fn ConstructionScript
  (Utilities|FlowControl|Sequence
    (:then_0
      (Variables|Default|SetDoor_Close (.z (Variables|/Script/Engine.SceneComponent|GetRelativeLocation (Variables|Default|GetDoor)))))
    (:then_1
      (Variables|Default|SetDoor_Close (- (.z (Variables|/Script/Engine.SceneComponent|GetRelativeLocation (Variables|Default|GetOpen_positioon))) 1.2e+02)))))