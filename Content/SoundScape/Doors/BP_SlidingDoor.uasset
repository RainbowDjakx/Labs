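; Sliding double door Blueprint that opens and closes two panels through separate open and close events.
; The construction script caches closed Y positions from LeftDoor and RightDoor, and derives open positions by offsetting the Left and Right components in opposite directions.
; The Mouvement timeline lerps each panel's relative Y between them, playing from start to open and reversing from end to close.
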(event Custom|Event_OpenDoor
  (bind _mouvementvalue (Timeline|Mouvement PlayFromStart)
    (:Update
      (Transformation|SetRelativeLocation (Variables|Default|GetLeftDoor) (Math|Vector|MakeVector 0.0 (Math|Float|Lerp (Variables|Position|GetDoor_Left_Close) (Variables|Position|GetDoor_Left_Open) _mouvementvalue) 0.0) false false)
      (Transformation|SetRelativeLocation (Variables|Default|GetRightDoor) (Math|Vector|MakeVector 0.0 (Math|Float|Lerp (Variables|Position|GetDoor_Right_Close) (Variables|Position|GetDoor_Right_Open) _mouvementvalue) 0.0) false false))))

(event Custom|Event_CloseDoor
  (bind _mouvementvalue (Timeline|Mouvement ReverseFromEnd)
    (:Update
      (Transformation|SetRelativeLocation (Variables|Default|GetLeftDoor) (Math|Vector|MakeVector 0.0 (Math|Float|Lerp (Variables|Position|GetDoor_Left_Close) (Variables|Position|GetDoor_Left_Open) _mouvementvalue) 0.0) false false)
      (Transformation|SetRelativeLocation (Variables|Default|GetRightDoor) (Math|Vector|MakeVector 0.0 (Math|Float|Lerp (Variables|Position|GetDoor_Right_Close) (Variables|Position|GetDoor_Right_Open) _mouvementvalue) 0.0) false false))))

(fn ConstructionScript
  (Utilities|FlowControl|Sequence
    (:then_0
      (Variables|Position|SetDoor_Left_Close (.y (Variables|/Script/Engine.SceneComponent|GetRelativeLocation (Variables|Default|GetLeftDoor)))))
    (:then_1
      (Variables|Position|SetDoor_Left_Open (+ (.y (Variables|/Script/Engine.SceneComponent|GetRelativeLocation (Variables|Default|GetLeft))) 5e+01)))
    (:then_2
      (Variables|Position|SetDoor_Right_Close (.y (Variables|/Script/Engine.SceneComponent|GetRelativeLocation (Variables|Default|GetRightDoor)))))
    (:then_3
      (Variables|Position|SetDoor_Right_Open (- (.y (Variables|/Script/Engine.SceneComponent|GetRelativeLocation (Variables|Default|GetRight))) 5e+01)))))