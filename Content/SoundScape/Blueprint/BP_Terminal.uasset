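; BP_Terminal is an interactable terminal that opens and closes a linked door when the player is authorised.
; Authorisation requires the player's key inventory component to pass checks for all three configured key IDs.
; Entering the display range turns the screen to its normal or red material based on authorisation, and leaving restores the default.
; Interacting repeats the key check, then toggles the door through its open and close events.
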(event OnComponentBeginOverlap(InteractionDisplayRange)
  (params (OverlappedComponent :type Primitive%20Component%20Object%20Reference) (OtherActor :type Actor%20Object%20Reference) (OtherComp :type Primitive%20Component%20Object%20Reference) (OtherBodyIndex :type Integer) (bFromSweep :type Boolean) (SweepResult :type Hit%20Result%20Structure%20%28by%20ref%29))
  (Utilities|Casting|CastToBp_Player OtherActor)
  (CallFunction|UpdateMaterial))

(event OnComponentEndOverlap(InteractionDisplayRange)
  (params (OverlappedComponent :type Primitive%20Component%20Object%20Reference) (OtherActor :type Actor%20Object%20Reference) (OtherComp :type Primitive%20Component%20Object%20Reference) (OtherBodyIndex :type Integer))
  (Utilities|Casting|CastToBp_Player OtherActor)
  (Rendering|Material|SetMaterialbyName (Variables|Default|GetStaticMeshComponent0) "Screen" "/Game/SoundScape/Props/Material/Screen.Screen"))

(event Custom|Update_Material
  (bind _is_granted (CallFunction|FuctionIsPlayerAutorise))
  (if _is_granted
    (Rendering|Material|SetMaterialbyName (Variables|Default|GetStaticMeshComponent0) "Screen" "/Game/SoundScape/Props/Material/M_Terminal_Screen.M_Terminal_Screen")
    (else
      (Rendering|Material|SetMaterialbyName (Variables|Default|GetStaticMeshComponent0) "Screen" "/Game/SoundScape/Props/Material/MI_Terminal_Screen_Red.MI_Terminal_Screen_Red"))))

(event EventOnInteraction
  (bind _is_granted (CallFunction|FuctionIsPlayerAutorise))
  (if _is_granted
    (if (Variables|State|GetIs_Open)
      (Default|EventCloseDoor (Variables|Reference|GetRef_Door))
      (Variables|State|SetIs_Open false)
      (else
        (Default|EventOpenDoor (Variables|Reference|GetRef_Door))
        (Variables|State|SetIs_Open true)))))

(event EventBeginPlay
  (bind _asbp_player (Utilities|Casting|CastToBp_Player (Game|GetPlayerCharacter 0)))
  (Variables|Reference|SetRef_player _asbp_player))

(event EventOnInteract
  (params (PlayerRef :type BP%20Third%20Person%20Character%20Object%20Reference) (IsObjectFree :type Boolean))
  (bind _is_granted (CallFunction|FuctionIsPlayerAutorise))
  (if _is_granted
    (if (Variables|State|GetIs_Open)
      (Default|EventCloseDoor (Variables|Reference|GetRef_Door))
      (Variables|State|SetIs_Open false)
      (else
        (Default|EventOpenDoor (Variables|Reference|GetRef_Door))
        (Variables|State|SetIs_Open true)))))

(fn ConstructionScript)

(fn FuctionIsPlayerAutorise
  (bind _is_present (Default|FuctionCheckKey (Variables|/Game/SoundScape/Player/Bp_Player.Bp_Player_C|GetBPC_keyInventory (Variables|Reference|GetRef_player)) (Variables|Configuration|GetKey_ID_1)))
  (bind _is_present_2 (Default|FuctionCheckKey (Variables|/Game/SoundScape/Player/Bp_Player.Bp_Player_C|GetBPC_keyInventory (Variables|Reference|GetRef_player)) (Variables|Configuration|GetKey_ID_2)))
  (bind _is_present_3 (Default|FuctionCheckKey (Variables|/Game/SoundScape/Player/Bp_Player.Bp_Player_C|GetBPC_keyInventory (Variables|Reference|GetRef_player)) (Variables|Configuration|GetKey_ID_3)))
  (if (Math|Boolean|ANDBoolean _is_present _is_present_2 _is_present_3)
    (return true)
    (else
      (return false))))