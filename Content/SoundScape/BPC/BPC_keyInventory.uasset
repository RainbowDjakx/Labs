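; BPC_keyInventory is a Blueprint component that stores the keys its owner carries in a KeyBag array.
; Two events add a key to the bag or remove one from it.
; A check function loops through the bag and returns true when the given key is present, otherwise false.
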(event Custom|Event_Add_Key
  (params (Input :type Integer))
  (Utilities|Array|Add (Variables|Default|GetKeyBag) Input))

(event Custom|Event_DeletKey
  (params (Key :type Integer))
  (Utilities|Array|RemoveItem (Variables|Default|GetKeyBag) Key))

(fn FuctionCheckKey
  (params (Key :type Integer))
  (for _array_element (Variables|Default|GetKeyBag)
    (if (== _array_element Key)
      (return true)))
  (return false))