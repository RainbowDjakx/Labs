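; Player component that lets Bp_Player pick up and release BP_Fuse items with a physics handle.
; The IA_Grab_Realease input toggles: a short camera line trace, with debug draw, finds a fuse and grabs the hit component.
; While grabbing, Tick moves the handle target just ahead of and slightly above the camera.
; Releasing frees the component and calls EventOnRealease on the stored fuse.
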(event Custom|Grab
  (params (Ref_Component :type Primitive%20Component%20Object%20Reference%20%28by%20ref%29) (Component%20Transform :type Transform))
  (Physics|Components|PhysicsHandle|GrabComponentatLocationwithRotation (Variables|/Game/SoundScape/Player/Bp_Player.Bp_Player_C|Getobjecthandle (Variables|Reference|GetRef_Player)) Ref_Component "None" (.location Component%20Transform) (.rotation Component%20Transform))
  (Variables|State|SetState_IsGrab true))

(event Custom|Ungrab
  (Physics|Components|PhysicsHandle|ReleaseComponent (Variables|/Game/SoundScape/Player/Bp_Player.Bp_Player_C|Getobjecthandle (Variables|Reference|GetRef_Player))))

(event Input|EnhancedActionEvents|EnhancedInputActionIA_Grab_Realease
  (params (ActionValue :type Boolean) (ElapsedSeconds :type Float%20%28double-precision%29) (TriggeredSeconds :type Float%20%28double-precision%29) (InputAction :type Input%20Action%20Object%20Reference :default "/Game/SoundScape/Player/Input/Action/IA_Grab_Realease.IA_Grab_Realease"))
  (bind _ref_player (Variables|Reference|GetRef_Player))
  (bind _camera_scop (Variables|/Game/SoundScape/Player/Bp_Player.Bp_Player_C|GetCamera_Scop _ref_player))
  (bind _returnvalue (Transformation|GetWorldLocation _camera_scop))
  (:Started
    (if (Variables|State|GetState_IsGrab)
      (CallFunction|Ungrab)
      (Default|EventonRealease (Variables|Reference|GetRef_Fusebp))
      (Variables|State|SetState_IsGrab false)
      (else
        (bind _outhit (Collision|LineTraceByChannel _returnvalue (+ _returnvalue (* (Math|Vector|GetForwardVector (Transformation|GetWorldRotation _camera_scop)) 2e+02)) "TraceTypeQuery1" true 0 "ForDuration"))
        (bind _asbp_fuse (Utilities|Casting|CastToBP_Fuse (.hitactor _outhit)))
        (Variables|Reference|SetRef_Fusebp _asbp_fuse)
        (Variables|Reference|SetRef_ItemGrab (.hitcomponent _outhit))
        (CallFunction|Grab (Variables|Reference|GetRef_ItemGrab) (Transformation|GetWorldTransform (Variables|Reference|GetRef_ItemGrab)))))))

(event EventBeginPlay
  (bind _asbp_player (Utilities|Casting|CastToBp_Player (Components|GetOwner)))
  (Variables|Reference|SetRef_Player _asbp_player))

(event EventTick
  (params (DeltaSeconds :type Float%20%28single-precision%29))
  (bind _ref_player (Variables|Reference|GetRef_Player))
  (bind _camera_scop (Variables|/Game/SoundScape/Player/Bp_Player.Bp_Player_C|GetCamera_Scop _ref_player))
  (bind _returnvalue (Transformation|GetWorldLocation _camera_scop))
  (bind _returnvalue_2 (Transformation|GetWorldRotation _camera_scop))
  (bind _returnvalue_3 (Math|Vector|GetForwardVector _returnvalue_2))
  (bind _returnvalue_4 (* _returnvalue_3 5e+01))
  (bind _returnvalue_5 (+ _returnvalue _returnvalue_4))
  (if (Variables|State|GetState_IsGrab)
    (Physics|Components|PhysicsHandle|SetTargetLocation (Variables|/Game/SoundScape/Player/Bp_Player.Bp_Player_C|Getobjecthandle (Variables|Reference|GetRef_Player)) (Math|Vector|MakeVector (.x _returnvalue_5) (.y _returnvalue_5) (+ (.z _returnvalue_5) 1e+01)))))