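; Player component that lets the player scan for speakers through a scope camera and retune their radio frequency.
; The highjack input toggles the scope camera and a looping timer that line-traces forward, with debug drawing, and sends an interact message to the hit actor.
; The select event stores a speaker and its frequency, and the HUD shows detection.
; Increase and decrease inputs push clamped frequency steps to the selected speaker's radio component.
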(event Custom|Event_Scan
  (if (Variables|State|GetIs_Scope)
    (bind _returnvalue (Utilities|Time|SetTimerbyEvent (delegate Custom|CustomEvent) 0.1 true))
    (Variables|Reference|SetRef_ScanTimer _returnvalue)
    (else
      (Utilities|Time|ClearandInvalidateTimerbyHandle (Variables|Reference|GetRef_ScanTimer)))))

(event Custom|CustomEvent
  (bind _ref_player (Variables|Reference|GetRef_Player))
  (bind _ref_player_2 (Variables|Reference|GetRef_Player))
  (bind _camera_scop (Variables|/Game/SoundScape/Player/Bp_Player.Bp_Player_C|GetCamera_Scop _ref_player))
  (bind _hud (Variables|/Game/SoundScape/Player/Bp_Player.Bp_Player_C|GetHUD _ref_player_2))
  (bind _returnvalue (Transformation|GetWorldLocation _camera_scop))
  (bind _outhit (Collision|LineTraceByChannel _returnvalue (+ _returnvalue (* (Math|Vector|GetForwardVector (Transformation|GetWorldRotation _camera_scop)) 2e+03)) "TraceTypeQuery1" false 0 "ForDuration" true "(R=0.854956,G=0.000000,B=1.000000,A=1.000000)" "(R=0.000000,G=0.887733,B=1.000000,A=1.000000)"))
  (Variables|State|SetIs_Speaker_Selected false)
  (Class|BPIRadioInteraction|FunctionInteract(Message) (.hitactor _outhit) (Variables|Reference|GetRef_Player) false)
  (if (Variables|State|GetIs_Speaker_Selected)
    (Default|EventDetecton _hud)
    (else
      (Default|EventDetectOff _hud))))

(event Custom|Event_SelectSpeaker
  (params (Speaker_Ref :type BP%20Wallspeaker%20Object%20Reference) (Frequences :type Float%20%28double-precision%29))
  (Variables|Reference|SetSpeaker%20Ref Speaker_Ref)
  (Variables|State|SetIs_Speaker_Selected true)
  (Variables|State|SetFrequence Frequences)
  (Default|EventChangeTexte (Variables|/Game/SoundScape/Player/Bp_Player.Bp_Player_C|GetHUD (Variables|Reference|GetRef_Player)) (Variables|State|GetFrequence)))

(event Custom|Event_Set_Ref_Item_Speaker
  (params (Input_Speaker :type BP%20Item%20Speaker%20Object%20Reference)))

(event Input|EnhancedActionEvents|EnhancedInputActionIA_Highjack
  (params (ActionValue :type Boolean) (ElapsedSeconds :type Float%20%28double-precision%29) (TriggeredSeconds :type Float%20%28double-precision%29) (InputAction :type Input%20Action%20Object%20Reference :default "/Game/SoundScape/Player/Input/Action/IA_Highjack.IA_Highjack"))
  (:Started
    (Variables|State|SetIs_Scope (not (Variables|State|GetIs_Scope)))
    (Default|EventChangeCamera (Variables|Reference|GetRef_Player) (Variables|State|GetIs_Scope))
    (CallFunction|EventScan)))

(event Input|EnhancedActionEvents|EnhancedInputActionIA_IncreaseFrequence
  (params (ActionValue :type Boolean) (ElapsedSeconds :type Float%20%28double-precision%29) (TriggeredSeconds :type Float%20%28double-precision%29) (InputAction :type Input%20Action%20Object%20Reference :default "/Game/SoundScape/Player/Input/Action/IA_IncreaseFrequence.IA_IncreaseFrequence"))
  (if (and (< (Variables|State|GetFrequence) 282.0) (Variables|State|GetIs_Speaker_Selected))
    (bind _output_get (Variables|State|SetFrequence (Math|Float|Clamp(Float) (+ (Variables|State|GetFrequence) 0.1) 1.5e+02 281.0)))
    (Default|EventSetFrequence (Variables|/Game/SoundScape/Blueprint/BP_Wallspeaker.BP_Wallspeaker_C|GetBPC_Radio (Variables|Reference|GetSpeaker%20Ref)) _output_get)))

(event Input|EnhancedActionEvents|EnhancedInputActionIA_DecreaseFrequence
  (params (ActionValue :type Boolean) (ElapsedSeconds :type Float%20%28double-precision%29) (TriggeredSeconds :type Float%20%28double-precision%29) (InputAction :type Input%20Action%20Object%20Reference :default "/Game/SoundScape/Player/Input/Action/IA_DecreaseFrequence.IA_DecreaseFrequence"))
  (if (and (> (Variables|State|GetFrequence) 149.0) (Variables|State|GetIs_Speaker_Selected))
    (bind _output_get (Variables|State|SetFrequence (Math|Float|Clamp(Float) (- (Variables|State|GetFrequence) 0.1) 1.5e+02 281.0)))
    (Default|EventSetFrequence (Variables|/Game/SoundScape/Blueprint/BP_Wallspeaker.BP_Wallspeaker_C|GetBPC_Radio (Variables|Reference|GetSpeaker%20Ref)) _output_get)))

(event EventBeginPlay
  (bind _asbp_player (Utilities|Casting|CastToBp_Player (Components|GetOwner)))
  (Variables|Reference|SetRef_Player _asbp_player))