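; BPC_Interaction is an actor component that lets the player interact with nearby objects.
; On BeginPlay it casts its owner to Bp_Player and stores it as a reference.
; The Interact input runs a stationary complex sphere trace on the Visibility channel, placed and sized by the player's InteractionCenter and InteractionDetection components, then sends OnInteractionMessage to the hit actor.
; Debug printing and trace drawing are left enabled.
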(event Input|EnhancedActionEvents|EnhancedInputActionIA_Interact
  (params (ActionValue :type Boolean) (ElapsedSeconds :type Float%20%28double-precision%29) (TriggeredSeconds :type Float%20%28double-precision%29) (InputAction :type Input%20Action%20Object%20Reference :default "/Game/SoundScape/Player/Input/Action/IA_Interact.IA_Interact"))
  (bind _ref_player (Variables|Default|GetRef_Player))
  (bind _interaction_center (Variables|/Game/SoundScape/Player/Bp_Player.Bp_Player_C|GetInteraction_center _ref_player))
  (bind _returnvalue (Transformation|GetWorldLocation _interaction_center))
  (:Started
    (Development|PrintString "Hello")
    (bind _outhit (Collision|SphereTraceByChannel _returnvalue _returnvalue (Components|Sphere|GetScaledSphereRadius (Variables|/Game/SoundScape/Player/Bp_Player.Bp_Player_C|GetInteraction%20Detection (Variables|Default|GetRef_Player))) "TraceTypeQuery1" true 0 "ForDuration"))
    (Class|BPIInteraction|OnInteraction(Message) (.hitactor _outhit))))

(event EventBeginPlay
  ;[1 0 0] Begin Play
  ;;[1 1 1] Set player
  (bind _asbp_player (Utilities|Casting|CastToBp_Player (Components|GetOwner)))
  (Variables|Default|SetRef_Player _asbp_player))