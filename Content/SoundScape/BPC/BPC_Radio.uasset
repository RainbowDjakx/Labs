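; Radio component that drives a tunable, four-track MetaSound on its owning actor.
; On BeginPlay it caches the owner's box and audio components, then feeds four waves into the MetaSound.
; Tuning clamps the frequency and sends it to the MetaSound; a key check tests it against a target band.
; A lookup returns speaker data from DT_SpeakerList by ID; the uncalled frequency setup writes only Frequence_Track_1.
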(event Custom|Event_Set_MetaSound
  (params (Input%20Meta%20sound :type Audio%20Component%20Object%20Reference))
  ;[0.4271 0.3817 0.1491] Setup
  (Variables|Default|SetRef_MetaSound Input%20Meta%20sound))

(event Custom|Event_Set_Hitbox
  (params (Inpu_Box_Colision :type Box%20Component%20Object%20Reference))
  ;[0.4271 0.3817 0.1491] Setup
  (Variables|Default|SetRef_Hitbox Inpu_Box_Colision))

(event Custom|Event_Setup_Sound
  ;[0.4271 0.3817 0.1491] Setup
  (Class|AudioComponent|SetWaveParameter (Variables|Default|GetRef_MetaSound) "Audio_Track_1" (Variables|Configuration|GetAudio%20input%201))
  (Class|AudioComponent|SetWaveParameter (Variables|Default|GetRef_MetaSound) "Audio_Track_2" (Variables|Configuration|GetAudio%20input%202))
  (Class|AudioComponent|SetWaveParameter (Variables|Default|GetRef_MetaSound) "Audio_Track_3" (Variables|Configuration|GetAudio%20input%203))
  (Class|AudioComponent|SetWaveParameter (Variables|Default|GetRef_MetaSound) "Audio_Track_4" (Variables|Configuration|GetAudio%20input%204)))

(event Custom|Event_Setup_Frequence
  ;[0.4271 0.3817 0.1491] Setup
  (Audio|Parameter|SetFloatParameter (Variables|Default|GetRef_MetaSound) "Frequence_Track_1" (Variables|Configuration|GetFrequence%201) :!class /Script/AudioExtensions.AudioParameterControllerInterface)
  (Audio|Parameter|SetFloatParameter (Variables|Default|GetRef_MetaSound) "Frequence_Track_1" (Variables|Configuration|GetFrequence%202) :!class /Script/AudioExtensions.AudioParameterControllerInterface)
  (Audio|Parameter|SetFloatParameter (Variables|Default|GetRef_MetaSound) "Frequence_Track_1" (Variables|Configuration|GetFrequence%203) :!class /Script/AudioExtensions.AudioParameterControllerInterface)
  (Audio|Parameter|SetFloatParameter (Variables|Default|GetRef_MetaSound) "Frequence_Track_1" (Variables|Configuration|GetFrequence%204) :!class /Script/AudioExtensions.AudioParameterControllerInterface))

(event Custom|Event_Set_Frequence
  (params (Frequence :type Float%20%28double-precision%29))
  (Variables|State|SetCurrent_Frequence (Math|Float|Clamp(Float) Frequence 1.5e+02 281.0))
  (Audio|Parameter|SetFloatParameter (Variables|Default|GetRef_MetaSound) "Frequence" (Variables|State|GetCurrent_Frequence) :!class /Script/AudioExtensions.AudioParameterControllerInterface))

(event EventBeginPlay
  ;[0.1398 0.4427 0.06059] Begin
  (CallFunction|EventSetHitbox (Actor|GetComponentbyClass (Components|GetOwner) "/Script/Engine.BoxComponent"))
  (CallFunction|EventSetMetaSound (Actor|GetComponentbyClass (Components|GetOwner) "/Script/Engine.AudioComponent"))
  (CallFunction|EventSetupSound))

(fn FunctionGetData
  (bind _outrownames (DataTable|GetDataTableRowNames "/Game/SoundScape/AudioData/DT_SpeakerList.DT_SpeakerList"))
  (for _array_element _outrownames
    (bind _returnvalue (Utilities|GetDataTableRow "/Game/SoundScape/AudioData/DT_SpeakerList.DT_SpeakerList" _array_element)
      (:then
        (if (== (Variables|Configuration|GetID_Speaker) (.id _returnvalue))
          (return (.speaker_name _returnvalue) (.frequence_track _returnvalue) (.track _returnvalue) (.static_track _returnvalue) (.resonance_station _returnvalue)))))))

(fn FuctionCheckKey
  (bind _current_frequence (Variables|State|GetCurrent_Frequence))
  (return (and (< _current_frequence (+ (Variables|Configuration|Getkey_frequence_max) 1.0)) (> _current_frequence (- (Variables|Configuration|Getkey_frequence_Min) 1.0)))))