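; BP_GrabCube is a prototype grabbable cube actor that can be dropped onto snap points.
; On interact, if it is free, it passes its mesh and itself to the player's grab event.
; Its Collision overlaps track a nearby BP_SnapPoint and print debug feedback.
; On release near one, it zeroes linear velocity and teleports to the snap position and rotation, keeping its scale.
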(event OnComponentBeginOverlap(Collision)
  (params (OverlappedComponent :type Primitive%20Component%20Object%20Reference) (OtherActor :type Actor%20Object%20Reference) (OtherComp :type Primitive%20Component%20Object%20Reference) (OtherBodyIndex :type Integer) (bFromSweep :type Boolean) (SweepResult :type Hit%20Result%20Structure%20%28by%20ref%29))
  (bind _asbp_snap_point (Utilities|Casting|CastToBP_SnapPoint OtherActor))
  (Variables|Default|SetSnapPointRef _asbp_snap_point)
  (Variables|Default|SetIsNearSnap true)
  (Development|PrintString (Utilities|GetDisplayName (Variables|Default|GetSnapPointRef))))

(event OnComponentEndOverlap(Collision)
  (params (OverlappedComponent :type Primitive%20Component%20Object%20Reference) (OtherActor :type Actor%20Object%20Reference) (OtherComp :type Primitive%20Component%20Object%20Reference) (OtherBodyIndex :type Integer))
  (if (== OtherActor (Variables|Default|GetSnapPointRef))
    (Variables|Default|SetIsNearSnap false)
    (Development|PrintString "NoSnap")))

(event Custom|EventOnRealease
  (bind _self self)
  (bind _snappointref (Variables|Default|GetSnapPointRef))
  (bind _snapposition (Variables|/Game/PROTOTYPE/GrabAndDrop/BP_SnapPoint.BP_SnapPoint_C|GetSnapPosition _snappointref))
  (if (Variables|Default|GetIsNearSnap)
    (Physics|SetPhysicsLinearVelocity (Variables|Default|GetStaticMeshComponent0 _self) "0, 0, 0" false "None")
    (Transformation|SetActorTransform _self (Math|Transform|MakeTransform (.location _snapposition) (.rotation _snapposition) (Transformation|GetActorScale3D)) false true)))

(event EventOnInteract
  (params (PlayerRef :type BP%20Third%20Person%20Character%20Object%20Reference) (IsObjectFree :type Boolean))
  (if IsObjectFree
    (Default|EventGrabObject PlayerRef (Variables|Default|GetStaticMeshComponent0) self)))

(fn ConstructionScript)