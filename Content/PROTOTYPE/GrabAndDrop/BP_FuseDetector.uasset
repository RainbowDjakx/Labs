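; BP_FuseDetector is a prototype trigger that fades a referenced spotlight on when a BP_Fuse enters its overlap box and off when it leaves.
; Begin and end overlap each start a looping timer that steps a normalised alpha, lerps it to intensity in lumens, and clears itself at the limit.
; Both timers share one handle, debug prints trace the state, and the construction script scales the box.
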(event OnComponentBeginOverlap(OverlapBox)
  (params (OverlappedComponent :type Primitive%20Component%20Object%20Reference) (OtherActor :type Actor%20Object%20Reference) (OtherComp :type Primitive%20Component%20Object%20Reference) (OtherBodyIndex :type Integer) (bFromSweep :type Boolean) (SweepResult :type Hit%20Result%20Structure%20%28by%20ref%29))
  ;[1 1 1] Turning the light on
  (Utilities|Casting|CastToBP_Fuse OtherActor)
  (Development|PrintString "Fuse Detected")
  (CallFunction|SetLightIntencity 0.0)
  (bind _returnvalue (Utilities|Time|SetTimerbyEvent (delegate Custom|EventLightOn) 0.1 true))
  (Variables|Default|SetTimerLight _returnvalue))

(event OnComponentEndOverlap(OverlapBox)
  (params (OverlappedComponent :type Primitive%20Component%20Object%20Reference) (OtherActor :type Actor%20Object%20Reference) (OtherComp :type Primitive%20Component%20Object%20Reference) (OtherBodyIndex :type Integer))
  ;[1 1 1] Turning Off The light
  (Utilities|Casting|CastToBP_Fuse OtherActor)
  (Development|PrintString "Fuse Remove")
  (CallFunction|SetLightIntencity 2.5e+02)
  (bind _returnvalue (Utilities|Time|SetTimerbyEvent (delegate Custom|EventLightOff) 0.1 true))
  (Variables|Default|SetTimerLight _returnvalue))

(event Custom|EventLightOff
  ;[1 1 1] Turning Off The light
  (bind _output_get (Variables|Default|SetNormaliseIntensity (- (Variables|Default|GetNormaliseIntensity) (Variables|Default|GetLightTurnigSpeed))))
  (Development|PrintString (Utilities|String|ToString(Float) _output_get) true true "(R=0.000000,G=0.660000,B=1.000000,A=1.000000)" 2.0 "light")
  (CallFunction|SetLightIntencity (Math|Float|Lerp 0.0 2.5e+02 _output_get))
  (if (<= (Math|Float|Lerp 0.0 2.5e+02 _output_get) 0.0)
    (CallFunction|EventKillLightTimer)))

(event Custom|EventKillLightTimer
  ;[1 1 1] Stop the light Update
  (Utilities|Time|ClearandInvalidateTimerbyHandle (Variables|Default|GetTimerLight)))

(event Custom|EventLightOn
  ;[1 1 1] Turning the light on
  (bind _output_get (Variables|Default|SetNormaliseIntensity (+ (Variables|Default|GetNormaliseIntensity) (Variables|Default|GetLightTurnigSpeed))))
  (Development|PrintString (Utilities|String|ToString(Float) _output_get) true true "(R=0.000000,G=0.660000,B=1.000000,A=1.000000)" 2.0 "light")
  (CallFunction|SetLightIntencity (Math|Float|Lerp 0.0 2.5e+02 _output_get))
  (if (>= (Math|Float|Lerp 0.0 2.5e+02 _output_get) 2.5e+02)
    (CallFunction|EventKillLightTimer)))

(event Custom|SetLightIntencity
  (params (Intensity :type Float%20%28double-precision%29))
  (Rendering|Components|Light|SetIntensity (Variables|Default|GetSpot%20Light%20Component) Intensity))

(event EventBeginPlay
  (bind _lightref (Variables|Default|GetLightRef))
  (bind _spotlightcomponent (Variables|/Script/Engine.SpotLight|GetSpotLightComponent _lightref))
  (Variables|Default|SetSpot%20Light%20Component _spotlightcomponent)
  (Class|LocalLightComponent|SetIntensityUnits _spotlightcomponent "Lumens"))

(fn ConstructionScript
  (Transformation|SetWorldScale3D (Variables|Default|GetOverlapBox) (Variables|Default|GetScale)))