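; BP_Radio is a prototype radio that starts playing its MSRadio audio on BeginPlay and responds to tuning.
; The construction script passes three track frequencies to MSRadio as float parameters, and an event forwards the incoming frequency the same way.
; A station function maps exact frequency matches to a station number, or 0 otherwise.
; Its second check repeats FrequencePiste1, so station 2 is never returned.
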(event Custom|Event_Radio_Frequens_In
  (params (Frequence :type Float%20%28double-precision%29))
  (Audio|Parameter|SetFloatParameter (Variables|Default|GetMS_Radio) "Frequence" Frequence :!class /Script/AudioExtensions.AudioParameterControllerInterface))

(event EventBeginPlay
  (Audio|Components|Audio|Play (Variables|Default|GetMS_Radio) 0.0))

(fn ConstructionScript
  (bind _ms_radio (Variables|Default|GetMS_Radio))
  (Audio|Parameter|SetFloatParameter _ms_radio "Frequence_Piste_1" (Variables|Default|GetFrequence_Piste_1) :!class /Script/Engine.AudioComponent)
  (Audio|Parameter|SetFloatParameter _ms_radio "Frequence_Piste_2" (Variables|Default|GetFrequence_Piste_2) :!class /Script/Engine.AudioComponent)
  (Audio|Parameter|SetFloatParameter _ms_radio "Frequence_Piste_3" (Variables|Default|GetFrequence_Piste_3) :!class /Script/Engine.AudioComponent))

(fn FuctionGetCurrentStation
  (if (== (Variables|Default|GetFrequence_Piste_1) (Variables|Default|GetFrequence))
    (return 1)
    (elif (== (Variables|Default|GetFrequence_Piste_1) (Variables|Default|GetFrequence))
      (return 2)
      (elif (== (Variables|Default|GetFrequence_Piste_3) (Variables|Default|GetFrequence))
        (return 3)
        (else
          (return 0))))))